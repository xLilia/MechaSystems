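; Orbit camera for mecha customization that spawns a Mecha_BP on BeginPlay and selects its body.
; Holding the wheel button rotates and pitches the view from mouse movement, while scrolling zooms the spring arm.
; Right click cycles the mecha component and aligns to its owner; holding left mouse repeats that alignment without cycling.
; Helper functions are defined outside this graph, and a vertical MoveZ call is left unwired.
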(event `self.ReceiveBeginPlay`
  ;[1 1 1] Start
  (bind _returnvalue (`|SpawnActorFromClass` "/Game/Blueprints/MechaCustomization/Mecha_BP.Mecha_BP_C" (`KismetMathLibrary.MakeTransform` (0.0 0.0 300.0)) "Undefined" "OverrideRootScale" null null))
  (`self.SelectMechaBody` _returnvalue))

(event `InputAxis|MouseWheelButton`
  (params (AxisValue :type "Float (single-precision)"))
  ;[1 1 1] Camera Movement
  (if (> AxisValue 0.0)
    (`self.RotateZ` (`self.GetInputAxisValue`) 2.0)
    (`self.PitchCamera` (`self.GetInputAxisValue`) -2.0)))

(event `InputAxis|MouseWheel`
  (params (AxisValue :type "Float (single-precision)"))
  ;[1 1 1] Camera Movement
  (`self.ZoomOutSpringArm` AxisValue 30.0 (`self.SpringArm`)))

(event `InputAction|MouseRightButton`
  (params (Key :type "Key Structure"))
  ;[1 1 1] Camera Movement
  (:`Pressed`
    (bind _returnvalue (`self.ScrollMechaComponentID` 1))
    (`self.AlignWithTarget` (`ActorComponent.GetOwner` _returnvalue) (1.0 0.0 1.0) :!label _label)))

(event `InputAxis|MouseRightDown`
  (params (AxisValue :type "Float (single-precision)"))
  ;[1 1 1] Camera Movement
)

(event `InputAxis|MouseLeftDown`
  (params (AxisValue :type "Float (single-precision)"))
  ;[1 1 1] Camera Movement
  (if (> AxisValue 0.0)
    (goto _label)))

(event `self.ReceiveTick`
  (params (DeltaSeconds :type "Float (single-precision)"))
  ;[1 1 1] Camera Movement
)

(fn `UserConstructionScript`)