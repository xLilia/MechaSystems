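; BP_CameraEditor is the camera actor for mecha customization, spawning a mecha body at its own transform on BeginPlay and selecting it.
; Holding the mouse wheel button rotates and pitches the view from mouse movement while CustomMouseInterface hides and locks the cursor; scrolling zooms the spring arm.
; Left click cycles component sockets and right click cycles components.
; Vertical move and target alignment calls are left unwired.
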(event `self.ReceiveBeginPlay`
  ;[1 1 1] START
  (`|ExecutionSequence`
    (:`then_0`
      (bind _returnvalue (`|SpawnActorFromClass` "/Game/Blueprints/MechaCustomization/mechaBody/MechaBody_BP.MechaBody_BP_C" (`self.GetTransform`) "Undefined" "OverrideRootScale" null null))
      (`self.SelectMechaBody` _returnvalue))))

(event `InputAxis|MouseWheelButton`
  (params (AxisValue :type "Float (single-precision)"))
  (bind _returnvalue (`GameplayStatics.GetPlayerController` 0))
  (bind _returnvalue_2 (`GameplayStatics.GetPlayerController` 0))
  (bind _custommouseinterface (`self.CustomMouseInterface`))
  (bind _custommouseinterface_2 (`self.CustomMouseInterface`))
  ;[1 1 1] Camera Movement
  ;;[1 1 1] Mouse Wheel
  (if (> AxisValue 0.0)
    (`self.RotateZ` (`self.GetInputAxisValue`) 2.0)
    (`self.PitchCamera` (`self.GetInputAxisValue`) -2.0)
    (`CustomMouseInterface.HideMouse` _custommouseinterface_2 _returnvalue_2)
    (`CustomMouseInterface.LockMousePosToCoord` _custommouseinterface_2 _returnvalue_2)
    (else
      (`CustomMouseInterface.ShowMouse` _custommouseinterface _returnvalue)
      (`CustomMouseInterface.UnlockMousePos` _custommouseinterface _returnvalue))))

(event `InputAxis|MouseWheel`
  (params (AxisValue :type "Float (single-precision)"))
  ;[1 1 1] Camera Movement
  ;;[1 1 1] Mouse Wheel
  (`self.ZoomOutSpringArm` AxisValue 30.0 (`self.SpringArm`)))

(event `InputAction|MouseLeftButton`
  (params (Key :type "Key Structure"))
  ;[1 1 1] Camera Movement
  ;;[1 1 1] Components
  (:`Pressed`
    (`self.ScrollMechaComponentSocket` 1)))

(event `self.ReceiveTick`
  (params (DeltaSeconds :type "Float (single-precision)"))
  ;[1 1 1] Camera Movement
)

(event `InputAction|MouseRightButton`
  (params (Key :type "Key Structure"))
  ;[1 1 1] Camera Movement
  ;;[1 1 1] Components
  (:`Pressed`
    (bind _returnvalue (`self.ScrollMechaComponent` 1))
    (`/Engine/EditorBlueprintResources/StandardMacros.IsValid` _returnvalue)))

(event `InputAxis|MouseRightDown`
  (params (AxisValue :type "Float (single-precision)"))
  ;[1 1 1] Camera Movement
  ;;[1 1 1] Components
)

(event `InputAxis|MouseLeftDown`
  (params (AxisValue :type "Float (single-precision)"))
  ;[1 1 1] Camera Movement
  ;;[1 1 1] Components
  (if (> AxisValue 0.0)
    _))

(fn `UserConstructionScript`)