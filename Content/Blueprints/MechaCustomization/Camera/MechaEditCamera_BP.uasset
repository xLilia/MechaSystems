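; Mecha customization camera that spawns a MechaBody_BP at its own transform on BeginPlay and selects it for editing.
; Holding the mouse wheel button rotates and pitches the view from mouse movement, and scrolling zooms the spring arm.
; Left click cycles component sockets; right click cycles components and aligns with the new component's owner using a multiplier that zeroes Y.
; Vertical panning logic is present but unconnected.
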(event `self.ReceiveBeginPlay`
  ;[1 1 1] Spawn Base
  (bind _returnvalue (`|SpawnActorFromClass` "/Game/Blueprints/MechaCustomization/MechaBody_BP.MechaBody_BP_C" (`self.GetTransform`) "Undefined" "OverrideRootScale" null null))
  (`self.SelectMechaBody` _returnvalue))

(event `InputAxis|MouseWheelButton`
  (params (AxisValue :type "Float (single-precision)"))
  ;[1 1 1] Camera Movement
  (if (> AxisValue 0.0)
    (`self.RotateZ` (`self.GetInputAxisValue`) 2.0)
    (`self.PitchCamera` (`self.GetInputAxisValue`) -2.0)))

(event `InputAxis|MouseWheel`
  (params (AxisValue :type "Float (single-precision)"))
  ;[1 1 1] Camera Movement
  (`self.ZoomOutSpringArm` AxisValue 30.0 (`self.SpringArm`)))

(event `InputAction|MouseLeftButton`
  (params (Key :type "Key Structure"))
  ;[1 1 1] Camera Movement
  (:`Pressed`
    (`self.ScrollMechaComponentSocket` 1)))

(event `InputAction|MouseRightButton`
  (params (Key :type "Key Structure"))
  ;[1 1 1] Camera Movement
  (:`Pressed`
    (bind _returnvalue (`self.ScrollMechaComponent` 1))
    (`self.AlignWithTarget` (`ActorComponent.GetOwner` _returnvalue) (1.0 0.0 1.0))))

(event `InputAxis|MouseRightDown`
  (params (AxisValue :type "Float (single-precision)"))
  ;[1 1 1] Camera Movement
)

(event `InputAxis|MouseLeftDown`
  (params (AxisValue :type "Float (single-precision)"))
  ;[1 1 1] Camera Movement
  (if (> AxisValue 0.0)
    _))

(event `self.ReceiveTick`
  (params (DeltaSeconds :type "Float (single-precision)"))
  ;[1 1 1] Camera Movement
)

(fn `UserConstructionScript`)