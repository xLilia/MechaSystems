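; BP_MechaHip is the hip component actor for mecha editing, showing a selection highlight when the hip is selected.
; After calling the parent Tick, it reads IsComponentSelected from MechaComponent every frame and shows or hides HipboneSelect and Hipbone1Select to match, without propagating to children.
; BeginPlay and overlap events are disabled stubs, and the construction script only calls its parent.
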(event `self.ReceiveTick`
  (params (DeltaSeconds :type "Float (single-precision)"))
  (bind _hipboneselect (`self.hipboneSelect`))
  (bind _hipbone1select (`self.hipbone1Select`))
  (`parent.ReceiveTick` DeltaSeconds)
  (if (`MechaComponent.isComponentSelected` (`self.MechaComponent`))
    (`SceneComponent.SetVisibility` _hipboneselect true false)
    (`SceneComponent.SetVisibility` _hipbone1select true false)
    (else
      (`SceneComponent.SetVisibility` _hipboneselect false false)
      (`SceneComponent.SetVisibility` _hipbone1select false false))))

(fn `UserConstructionScript`
  (`parent.UserConstructionScript`))