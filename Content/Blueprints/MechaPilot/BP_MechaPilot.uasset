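; BP_MechaPilot is the player-controlled mecha pilot, turning input into look, movement and interaction.
; Mouse and move axes feed LookX, LookY, MoveForward and MoveRight, with vertical look given a negative speed.
; Pressing E_interact calls InteractionEventTrigger, passing the pressed key's display name as the event string and the pilot as instigator.
; BeginPlay, Tick, overlap and the construction script do nothing.
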(event `InputAxis|MouseY`
  (params (AxisValue :type "Float (single-precision)"))
  ;[1 1 1] Movement
  (`self.LookY` AxisValue -1.0))

(event `InputAxis|MoveForward`
  (params (AxisValue :type "Float (single-precision)"))
  ;[1 1 1] Movement
  (`self.MoveForward` AxisValue))

(event `InputAxis|MouseX`
  (params (AxisValue :type "Float (single-precision)"))
  ;[1 1 1] Movement
  (`self.LookX` AxisValue))

(event `InputAxis|MoveRight`
  (params (AxisValue :type "Float (single-precision)"))
  ;[1 1 1] Movement
  (`self.MoveRight` AxisValue))

(event `InputAction|E_interact`
  (params (Key :type "Key Structure"))
  (:`Pressed`
    (`InteractionEventTrigger.TriggerInteractionEvent` (`self.InteractionEventTrigger`) (`KismetTextLibrary.Conv_TextToString` (`KismetInputLibrary.Key_GetDisplayName` Key)) self)))

(fn `UserConstructionScript`)